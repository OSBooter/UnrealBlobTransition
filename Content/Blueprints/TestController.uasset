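; Test player controller that toggles game pause through an animated TransitionSlidInOut slide widget.
; On BeginPlay it creates the widget, adds it to the viewport and sets Game and UI input focused on it.
; The Pause input is ignored while the widget animates.
; Pausing calls ClosePause and pauses immediately, while unpausing calls OpenPause and waits briefly before resuming, with debug prints for both.
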(event `self.ReceiveBeginPlay`
  ;[1 1 1] This sends the animation info to the widget
  (bind _returnvalue (`|CreateWidget` "/Game/UI/TransitionSlidInOut.TransitionSlidInOut_C"))
  (`WidgetBlueprintLibrary.SetInputMode_GameAndUIEx` self _returnvalue)
  (bind _output_get (set `self.UIRef Pause` _returnvalue))
  (`UserWidget.AddToViewport` _output_get 0))

(event `InputAction|Pause` :paused true
  (params (Key :type "Key Structure"))
  ;[1 1 1] This sends the animation info to the widget
  (:`Pressed`
    (if (`UserWidget.IsAnyAnimationPlaying` (stale `self.ReceiveBeginPlay` _returnvalue))
      _
      (elif (`GameplayStatics.IsGamePaused`)
        (`/Game/UI/TransitionSlidInOut.Open Pause` (stale `self.ReceiveBeginPlay` _returnvalue))
        (`KismetSystemLibrary.Delay` 0.5)
        (`GameplayStatics.SetGamePaused` false)
        (`KismetSystemLibrary.PrintString` "Set Game Unpaused")
        (else
          (`/Game/UI/TransitionSlidInOut.Close Pause` (stale `self.ReceiveBeginPlay` _returnvalue))
          (`GameplayStatics.SetGamePaused` true)
          (`KismetSystemLibrary.PrintString` "Set Game Paused"))))))

(fn `UserConstructionScript`)